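; BPBall is the ball for a paddle game in the style of Pong, launched on BeginPlay by a single diagonal force on its physics sphere.
; Hits on a player or enemy paddle scale its velocity up and play the paddle sound, while other hits play the wall sound.
; Both sounds play at the player controller's location, and every hit briefly flashes the ball red before restoring white.
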(event `self.ReceiveBeginPlay`
  ;[1 1 1] Gives the ball a impulse towards the player
  (`PrimitiveComponent.AddForce` (`self.Sphere`) (100.0 100.0 0.0) "None" false))

(event `self.Sphere.OnComponentHit`
  (params (HitComponent :type "PrimitiveComponent Object Reference") (OtherActor :type "Actor Object Reference") (OtherComp :type "PrimitiveComponent Object Reference") (NormalImpulse :type "Vector Structure") (Hit :type "HitResult Structure (by ref)"))
  (bind _sphere (`self.Sphere`))
  (bind _returnvalue (`self.K2_GetActorLocation` (`GameplayStatics.GetPlayerController` 0)))
  ;[1 1 1] Only increases the ball speed if the hit was on one of the paddles.
  (cast `PlayerPaddle` OtherActor
    (:`then`
      (`PrimitiveComponent.SetPhysicsLinearVelocity` _sphere (* (`SceneComponent.GetComponentVelocity` _sphere) 1.15) false "None" :!label _label)
      ;[1 1 1] Plays the correct sound and makes the ball blink red
      (`GameplayStatics.PlaySoundAtLocation` "/Game/Sounds/paddlehit.paddlehit" _returnvalue (struct) 1.0 1.0 0.0 null null null))
    (:`CastFailed`
      (cast `EnemyPaddle` OtherActor
        (:`then`
          (goto _label))
        (:`CastFailed`
          (`GameplayStatics.PlaySoundAtLocation` "/Game/Sounds/wallhit.wallhit" _returnvalue (struct) 1.0 1.0 0.0 null null null)))))
  (`PrimitiveComponent.SetMaterial` (`self.Sphere`) 0 "/Game/Materials/MatRed.MatRed")
  (`KismetSystemLibrary.Delay` 0.1)
  (`PrimitiveComponent.SetMaterial` (`self.Sphere`) 0 "/Game/Materials/MatWhite.MatWhite"))

(fn `UserConstructionScript`)